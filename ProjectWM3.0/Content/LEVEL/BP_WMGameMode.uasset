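; Game mode that splits joining players into two teams, each spawning at its own house.
; PostLogin writes NextTeamIndex to the player's BP_WMPlayerState, restarts them at the HOUSE1 or HOUSE2 tagged player start, then toggles the index between 1 and 2.
; The ChoosePlayerStart override picks the house start from the stored TeamIndex, so spawns that use it stay on the team's side.
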(event `self.K2_PostLogin`
  (params (NewPlayer :type "PlayerController Object Reference"))
  (bind _nextteamindex (`self.NextTeamIndex`))
  (bind _asbp_wmplayer_state (cast `/Game/LEVEL/BP_WMPlayerState` (`Controller.PlayerState` NewPlayer)))
  (set `/Game/LEVEL/BP_WMPlayerState.TeamIndex` _nextteamindex _asbp_wmplayer_state)
  (if (== _nextteamindex 1)
    (`self.RestartPlayerAtPlayerStart` NewPlayer (`self.K2_FindPlayerStart` NewPlayer "HOUSE1"))
    (set `self.NextTeamIndex` 2)
    (else
      (`self.RestartPlayerAtPlayerStart` NewPlayer (`self.K2_FindPlayerStart` NewPlayer "HOUSE2"))
      (set `self.NextTeamIndex` 1))))

(fn `ChoosePlayerStart`
  (params (Player :type "Controller Object Reference"))
  (returns (ReturnValue :type "Actor Object Reference"))
  (bind _asbp_wmplayer_state (cast `/Game/LEVEL/BP_WMPlayerState` (`Controller.PlayerState` Player)))
  (if (== (`/Game/LEVEL/BP_WMPlayerState.TeamIndex` _asbp_wmplayer_state) 1)
    (return (`self.K2_FindPlayerStart` Player "HOUSE1"))
    (else
      (return (`self.K2_FindPlayerStart` Player "HOUSE2")))))

(fn `UserConstructionScript`)