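; Trash spawner actor that scatters TrashCount copies of each of four trash Blueprints across six box zones on BeginPlay.
; The construction script hard-codes the position and extent of each zone, including Livingroom.
; Each spawn takes a random point using center and extent from separate random BoxComponent picks, so the two can mismatch.
; Colliding spawns retry in an unbounded loop until one succeeds, with no authority check.
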(event `self.ReceiveBeginPlay`
  (bind _outitem (`KismetArrayLibrary.Array_Random` (`self.K2_GetComponentsByClass` "/Script/Engine.BoxComponent")))
  (bind _returnvalue (not (`self.SpawnSucceeded`)))
  (bind _returnvalue_2 (`SceneComponent.K2_GetComponentLocation` _outitem))
  (bind _returnvalue_3 (`BoxComponent.GetScaledBoxExtent` _outitem))
  (for _ (range (`self.TrashCount`))
    (set `self.SpawnSucceeded` false)
    (while _returnvalue
      (bind _returnvalue_4 (`|SpawnActorFromClass` "/Game/Fab/Trash/T/BP_Trash1.BP_Trash1_C" (`KismetMathLibrary.MakeTransform` (`KismetMathLibrary.RandomPointInBoundingBox` _returnvalue_2 _returnvalue_3)) "AdjustIfPossibleButDontSpawnIfColliding" "MultiplyWithRoot" null null))
      (`/Engine/EditorBlueprintResources/StandardMacros.IsValid` _returnvalue_4
        (:`Is Valid`
          (set `self.SpawnSucceeded` true))))
    (set `self.SpawnSucceeded` false)
    (while _returnvalue
      (bind _returnvalue_5 (`|SpawnActorFromClass` "/Game/Fab/Trash/T/BP_Trash2.BP_Trash2_C" (`KismetMathLibrary.MakeTransform` (`KismetMathLibrary.RandomPointInBoundingBox` _returnvalue_2 _returnvalue_3)) "AdjustIfPossibleButDontSpawnIfColliding" "MultiplyWithRoot" null null))
      (`/Engine/EditorBlueprintResources/StandardMacros.IsValid` _returnvalue_5
        (:`Is Valid`
          (set `self.SpawnSucceeded` true))))
    (set `self.SpawnSucceeded` false)
    (while _returnvalue
      (bind _returnvalue_6 (`|SpawnActorFromClass` "/Game/Fab/Trash/T/BP_Trash3.BP_Trash3_C" (`KismetMathLibrary.MakeTransform` (`KismetMathLibrary.RandomPointInBoundingBox` _returnvalue_2 _returnvalue_3)) "AdjustIfPossibleButDontSpawnIfColliding" "MultiplyWithRoot" null null))
      (`/Engine/EditorBlueprintResources/StandardMacros.IsValid` _returnvalue_6
        (:`Is Valid`
          (set `self.SpawnSucceeded` true))))
    (set `self.SpawnSucceeded` false)
    (while _returnvalue
      (bind _returnvalue_7 (`|SpawnActorFromClass` "/Game/Fab/Trash/T/BP_Trash4.BP_Trash4_C" (`KismetMathLibrary.MakeTransform` (`KismetMathLibrary.RandomPointInBoundingBox` _returnvalue_2 _returnvalue_3)) "AdjustIfPossibleButDontSpawnIfColliding" "MultiplyWithRoot" null null))
      (`/Engine/EditorBlueprintResources/StandardMacros.IsValid` _returnvalue_7
        (:`Is Valid`
          (set `self.SpawnSucceeded` true))))))

(fn `UserConstructionScript`
  (bind _livingroom (`self.Livingroom`))
  (bind _spawnzone_2 (`self.SpawnZone_2`))
  (bind _spawnzone_3 (`self.SpawnZone_3`))
  (bind _spawnzone_4 (`self.SpawnZone_4`))
  (bind _spawnzone_5 (`self.SpawnZone_5`))
  (bind _spawnzone_6 (`self.SpawnZone_6`))
  (`SceneComponent.K2_SetRelativeLocation` _livingroom (`KismetMathLibrary.MakeVector` 3080.0 -1565.0 10.0) false false)
  (`BoxComponent.SetBoxExtent` _livingroom (`KismetMathLibrary.MakeVector` 1000.0 900.0 8.0) false)
  (`SceneComponent.K2_SetRelativeLocation` _spawnzone_2 (`KismetMathLibrary.MakeVector` 3080.0 935.0 10.0) false false)
  (`BoxComponent.SetBoxExtent` _spawnzone_2 (`KismetMathLibrary.MakeVector` 1000.0 1200.0 8.0) false)
  (`SceneComponent.K2_SetRelativeLocation` _spawnzone_3 (`KismetMathLibrary.MakeVector` 880.0 -1565.0 10.0) false false)
  (`BoxComponent.SetBoxExtent` _spawnzone_3 (`KismetMathLibrary.MakeVector` 1000.0 900.0 8.0) false)
  (`SceneComponent.K2_SetRelativeLocation` _spawnzone_4 (`KismetMathLibrary.MakeVector` 880.0 935.0 10.0) false false)
  (`BoxComponent.SetBoxExtent` _spawnzone_4 (`KismetMathLibrary.MakeVector` 1000.0 1200.0 8.0) false)
  (`SceneComponent.K2_SetRelativeLocation` _spawnzone_5 (`KismetMathLibrary.MakeVector` -2320.0 -1565.0 10.0) false false)
  (`BoxComponent.SetBoxExtent` _spawnzone_5 (`KismetMathLibrary.MakeVector` 1400.0 900.0 8.0) false)
  (`SceneComponent.K2_SetRelativeLocation` _spawnzone_6 (`KismetMathLibrary.MakeVector` -2320.0 935.0 10.0) false false)
  (`BoxComponent.SetBoxExtent` _spawnzone_6 (`KismetMathLibrary.MakeVector` 1400.0 1200.0 8.0) false))